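; BP_HitPlatform is an actor that takes damage when the third-person character hits its cube and destroys itself once its health component allows.
; The Cube's hit event casts the other actor to BP_ThirdPersonCharacter, then subtracts a fixed amount from the HealthComponent's Health.
; It then asks the component whether it can be destroyed, either destroying the actor or printing the remaining health.
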(event OnComponentHit(Cube)
  (params (HitComponent :type Primitive%20Component%20Object%20Reference) (OtherActor :type Actor%20Object%20Reference) (OtherComp :type Primitive%20Component%20Object%20Reference) (NormalImpulse :type Vector :default "0, 0, 0") (Hit :type Hit%20Result%20Structure%20%28by%20ref%29))
  (bind _health_component (Variables|Default|GetHealth%20Component))
  (if (.bSuccess (Utilities|Casting|CastToBP_ThirdPersonCharacter OtherActor))
    (Variables|/Script/TheoryRepository.HealthComponent|SetHealth _health_component (- (Variables|/Script/TheoryRepository.HealthComponent|GetHealth _health_component) 2e+01))
    (if (Class|HealthComponent|CanItbeDestroyed (Variables|Default|GetHealth%20Component))
      (Actor|DestroyActor)
      (else
        (Development|PrintString (Utilities|String|Append "Healt Remaining: " (Utilities|String|ToString(Float) (Variables|/Script/TheoryRepository.HealthComponent|GetHealth _health_component))))))))

(event EventBeginPlay)

(event Collision|EventActorBeginOverlap
  (params (OtherActor :type Actor%20Object%20Reference)))

(event EventTick
  (params (DeltaSeconds :type Float%20%28single-precision%29)))

(fn ConstructionScript)