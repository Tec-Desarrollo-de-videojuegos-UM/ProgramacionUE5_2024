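; MyHitPlatform is a platform that wears down while a BP_ThirdPersonCharacter overlaps its box collider and eventually destroys itself.
; Begin overlap starts a Delay-based loop that calls Damage on its Health once per second until IsDestroyable returns true.
; End overlap by the character clears the IsToaching flag to stop the loop, while begin overlap sets it for any actor before the character cast.
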(event OnComponentEndOverlap(BoxCollider)
  (params (OverlappedComponent :type Primitive%20Component%20Object%20Reference) (OtherActor :type Actor%20Object%20Reference) (OtherComp :type Primitive%20Component%20Object%20Reference) (OtherBodyIndex :type Integer))
  (Utilities|Casting|CastToBP_ThirdPersonCharacter OtherActor)
  (Variables|Default|SetisToaching false))

(event OnComponentBeginOverlap(BoxCollider)
  (params (OverlappedComponent :type Primitive%20Component%20Object%20Reference) (OtherActor :type Actor%20Object%20Reference) (OtherComp :type Primitive%20Component%20Object%20Reference) (OtherBodyIndex :type Integer) (bFromSweep :type Boolean) (SweepResult :type Hit%20Result%20Structure%20%28by%20ref%29))
  (bind _health (Variables|Default|GetHealth))
  (bind _output_get (Variables|Default|SetisToaching true))
  (Utilities|Casting|CastToBP_ThirdPersonCharacter OtherActor :!label _label)
  (if _output_get
    (Class|HealthComponent|Damage _health)
    (bind _returnvalue (Class|HealthComponent|IsDestroyable _health))
    (if _returnvalue
      (Actor|DestroyActor)
      (else
        (Utilities|FlowControl|Delay 1.0)
        (goto _label)))))

(fn ConstructionScript)