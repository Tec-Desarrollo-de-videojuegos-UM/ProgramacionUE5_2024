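; Game state Blueprint that runs a game timer and displays its elapsed time on screen.
; On BeginPlay it starts the TimerManager, creates that manager's TimerWidget class, stores the instance back on the manager and adds it to the viewport.
; Each Tick, while the timer runs and the widget is valid, it pushes the elapsed time into the widget's text.
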(event EventBeginPlay
  (Class|TimerManagerComponent|StartTimer (Variables|Default|GetTimerManager))
  (bind _returnvalue (UserInterface|CreateWidget (Variables|/Script/TheoryRepository.TimerManagerComponent|GetTimerWidgetClass (Variables|Default|GetTimerManager))))
  (bind _astimer_widget (Utilities|Casting|CastToTimerWidget _returnvalue))
  (bind _output_get (Variables|/Script/TheoryRepository.TimerManagerComponent|SettimerWidgetInstance (Variables|Default|GetTimerManager) _astimer_widget))
  (UserInterface|Viewport|AddtoViewport _output_get 0))

(event EventTick
  (params (DeltaSeconds :type Float%20%28single-precision%29))
  (bind _timermanager (Variables|Default|GetTimerManager))
  (bind _timerwidgetinstance (Variables|/Script/TheoryRepository.TimerManagerComponent|GettimerWidgetInstance _timermanager))
  (if (Variables|/Script/TheoryRepository.TimerManagerComponent|GetbIsTimerRunning (Variables|Default|GetTimerManager))
    (Utilities|IsValid _timerwidgetinstance
      (:Is%20Valid
        (Class|TimerWidget|UpdateTimerText _timerwidgetinstance (Class|TimerManagerComponent|GetTimeElpased (Variables|Default|GetTimerManager)))))))

(fn ConstructionScript)