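; Door actor that swings open and closed around its yaw axis when its Interact event fires.
; BeginPlay caches the starting rotation and derives the end rotation by adding RotateToPoint to the yaw.
; Interact alternates through a FlipFlop between playing and reversing the RotateObject timeline, whose Alpha lerps the actor between the two rotations.
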(event EventBeginPlay
  (|CallParentFunction)
  (bind _output_get (Variables|Default|SetInitRotator (Transformation|GetActorRotation)))
  (Variables|Default|SetFinalRotator (Math|Rotator|MakeRotator (.Roll (Math|Rotator|BreakRotator _output_get)) (.Pitch (Math|Rotator|BreakRotator _output_get)) (+ (.Yaw (Math|Rotator|BreakRotator _output_get)) (Variables|Default|GetRotateToPoint)))))

(event Collision|EventActorBeginOverlap
  (params (OtherActor :type Actor%20Object%20Reference))
  (|CallParentFunction OtherActor) ; This node is disabled and will not be called.\nDrag off pins to build functionality.
)

(event EventTick
  (params (DeltaSeconds :type Float%20%28single-precision%29))
  (|CallParentFunction DeltaSeconds) ; This node is disabled and will not be called.\nDrag off pins to build functionality.
)

(event EventInteract
  (bind _rotateobject (Variables|Default|GetRotateObject))
  (Utilities|FlowControl|FlipFlop
    (:A
      (Audio|Components|Audio|Play _rotateobject))
    (:B
      (Utilities|String|Reverse _rotateobject))))

(fn ConstructionScript
  (|CallParentFunction))