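; BP_Platform is an interactable platform actor that moves between its start location and an offset point each time it is interacted with.
; On BeginPlay it stores its initial location and computes the destination by adding PointToMove.
; Interact uses a FlipFlop to alternately play and reverse the MoveObject timeline, whose Alpha lerps the actor's location between the two points without sweeping.
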(event EventBeginPlay
  (|CallParentFunction)
  (bind _output_get (Variables|Default|SetInitPosition (Transformation|GetActorLocation)))
  (Variables|Default|SetFinalPosition (+ _output_get (Variables|Default|GetPointToMove))))

(event Collision|EventActorBeginOverlap
  (params (OtherActor :type Actor%20Object%20Reference))
  (|CallParentFunction OtherActor) ; This node is disabled and will not be called.\nDrag off pins to build functionality.
)

(event EventTick
  (params (DeltaSeconds :type Float%20%28single-precision%29))
  (|CallParentFunction DeltaSeconds) ; This node is disabled and will not be called.\nDrag off pins to build functionality.
)

(event EventInteract
  (bind _moveobject (Variables|Default|GetMoveObject))
  (Utilities|FlowControl|FlipFlop
    (:A
      (Audio|Components|Audio|Play _moveobject))
    (:B
      (Utilities|String|Reverse _moveobject))))

(fn ConstructionScript
  (|CallParentFunction))