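; BP_Button is a trigger actor that marks a Character's controller as able to interact while that Character is inside its Box.
; On begin overlap it calls SetCanInteractMessage on the controller, passing its target actor, NPC, target point and move time.
; On end overlap it sends the same message with default values, withdrawing the interaction.
; The button only relays this data and performs no interaction or movement itself.
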(event OnComponentBeginOverlap(Box)
  (params (OverlappedComponent :type Primitive%20Component%20Object%20Reference) (OtherActor :type Actor%20Object%20Reference) (OtherComp :type Primitive%20Component%20Object%20Reference) (OtherBodyIndex :type Integer) (bFromSweep :type Boolean) (SweepResult :type Hit%20Result%20Structure%20%28by%20ref%29))
  (bind _ascharacter (Utilities|Casting|CastToCharacter OtherActor))
  (Class|BPIInteractable|SetCanInteract(Message) (Pawn|GetController _ascharacter) true (Variables|Default|GetActor%20to%20Interact) (Variables|Default|GetNPC) (Variables|Default|GetTargetPoint) (Variables|Default|GetTime%20to%20Move)))

(event OnComponentEndOverlap(Box)
  (params (OverlappedComponent :type Primitive%20Component%20Object%20Reference) (OtherActor :type Actor%20Object%20Reference) (OtherComp :type Primitive%20Component%20Object%20Reference) (OtherBodyIndex :type Integer))
  (bind _ascharacter (Utilities|Casting|CastToCharacter OtherActor))
  (Class|BPIInteractable|SetCanInteract(Message) (Pawn|GetController _ascharacter) false 0 0 0 0.0))

(fn ConstructionScript)