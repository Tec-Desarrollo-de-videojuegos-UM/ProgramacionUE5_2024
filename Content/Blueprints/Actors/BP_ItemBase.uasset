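; BP_ItemBase is an item base actor that, as scripted, repeatedly fires through its BulletSystem.
; From BeginPlay it loops on Shoot, waiting longer after a successful shot than after a failed one before trying again.
; An unconnected debug chain calls ChangeName and a looping ChangeAmount with printed results, but never runs.
; Tick and the construction script are empty.
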(event EventBeginPlay
  (bind _returnvalue (Class|BulletSystem|Shoot (Variables|Default|GetBulletSystem) :!label _label))
  (if _returnvalue
    (Utilities|FlowControl|Delay 3.0)
    (goto _label)
    (else
      (Utilities|FlowControl|Delay 1.0)
      (goto _label))))

(event EventTick
  (params (DeltaSeconds :type Float%20%28single-precision%29)))

(fn ConstructionScript)