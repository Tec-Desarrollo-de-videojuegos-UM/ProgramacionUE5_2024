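; AI controller for enemy NPCs that runs the BT_NPC behavior tree on BeginPlay and feeds it perception results through the blackboard.
; Perception updates store any BP_TopDownCharacter in PlayerToChase, stopping the loop at the first actor that fails the cast.
; Target perception updates write the stimulus's SuccessfullySensed flag straight into StopToChase, so it is true while sensed despite its name.
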(event OnPerceptionUpdated(AIPerception)
  (params (UpdatedActors :type Array%20of%20Actor%20Object%20References))
  (for _array_element UpdatedActors
    (bind _asbp_top_down_character (Utilities|Casting|CastToBP_TopDownCharacter _array_element))
    (AI|Components|Blackboard|SetValueasObject (AI|GetBlackboard 0) (Utilities|Name|MakeLiteralName "PlayerToChase") _asbp_top_down_character)))

(event OnTargetPerceptionUpdated(AIPerception)
  (params (Actor :type Actor%20Object%20Reference) (Stimulus :type AI%20Stimulus%20Structure))
  (AI|Components|Blackboard|SetValueasBool (AI|GetBlackboard 0) (Utilities|Name|MakeLiteralName "StopToChase") (.bSuccessfullySensed (Utilities|Struct|BreakAIStimulus Stimulus))))

(event EventBeginPlay
  (AI|RunBehaviorTree "/Game/Blueprints/NPc/BT_NPC.BT_NPC"))

(fn ConstructionScript)