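; BP_HitPlatform is a platform that takes damage whenever the third-person character enters its trigger box.
; Each overlap subtracts a fixed amount from its own Health and calls HealthStatus on it.
; If the Destruction flag is then set, the platform destroys itself; otherwise it prints the remaining health on screen.
; The end-overlap event only casts to the character and does nothing further.
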(event OnComponentBeginOverlap(TriggerBox)
  (params (OverlappedComponent :type Primitive%20Component%20Object%20Reference) (OtherActor :type Actor%20Object%20Reference) (OtherComp :type Primitive%20Component%20Object%20Reference) (OtherBodyIndex :type Integer) (bFromSweep :type Boolean) (SweepResult :type Hit%20Result%20Structure%20%28by%20ref%29))
  (bind _health (Variables|Default|GetHealth))
  (Utilities|Casting|CastToBP_ThirdPersonCharacter OtherActor)
  (Variables|/Script/TheoryRepository.HealthComponent|Sethealth _health (- (Variables|/Script/TheoryRepository.HealthComponent|Gethealth _health) 25))
  (Class|HealthComponent|HealthStatus _health)
  (if (Variables|/Script/TheoryRepository.HealthComponent|Getdestruction _health)
    (Actor|DestroyActor)
    (else
      (Development|PrintString (Utilities|String|ToString(Integer) (Variables|/Script/TheoryRepository.HealthComponent|Gethealth _health)) true true "(R=0.000000,G=0.660000,B=1.000000,A=1.000000)" 6.0))))

(event OnComponentEndOverlap(TriggerBox)
  (params (OverlappedComponent :type Primitive%20Component%20Object%20Reference) (OtherActor :type Actor%20Object%20Reference) (OtherComp :type Primitive%20Component%20Object%20Reference) (OtherBodyIndex :type Integer))
  (Utilities|Casting|CastToBP_ThirdPersonCharacter OtherActor))

(event EventBeginPlay)

(event Collision|EventActorBeginOverlap
  (params (OtherActor :type Actor%20Object%20Reference)))

(event EventTick
  (params (DeltaSeconds :type Float%20%28single-precision%29)))

(fn ConstructionScript)